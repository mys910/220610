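; BP_MobSpwan is a spawner actor that repeatedly spawns mobs at its Arrow component's transform, switching mob type as time passes.
; Tick accumulates elapsed time and uses DoOnce gates to fire Lv1 during the first minute and Lv2 afterwards.
; Lv1 starts a looping timer by function name for the first mob class; Lv2 clears it and starts one for the second class.
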(event `self.ReceiveTick`
  (params (DeltaSeconds :type "Float (single-precision)"))
  (set `self.Time` (+ DeltaSeconds (`self.Time`)))
  (if (<= (`self.Time`) 60.0)
    (`/Engine/EditorBlueprintResources/StandardMacros.DoOnce` false
      (:`Completed`
        (`self.Lv1`)))
    (else
      (`/Engine/EditorBlueprintResources/StandardMacros.DoOnce` false
        (:`Completed`
          (`self.Lv2`))))))

(event `Lv1`
  (`KismetSystemLibrary.K2_SetTimer` null "MobSpawn" 3.0 true))

(event `Lv2`
  (`KismetSystemLibrary.K2_ClearTimer` null "MobSpawn")
  (`KismetSystemLibrary.K2_SetTimer` null "MobSpawn2" 3.0 true))

(fn `MobSpawn`
  (`|SpawnActorFromClass` (`self.SpawnMob`) (`SceneComponent.K2_GetComponentToWorld` (`self.Arrow`)) "Undefined" "OverrideRootScale" null null))

(fn `MobSpawn2`
  (`|SpawnActorFromClass` (`self.SpawnMob2`) (`SceneComponent.K2_GetComponentToWorld` (`self.Arrow`)) "Undefined" "OverrideRootScale" null null))

(fn `UserConstructionScript`)