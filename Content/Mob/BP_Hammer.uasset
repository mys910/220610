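; BP_Hammer is an actor that orbits a target actor and damages what it touches, sparing the player pawn.
; Tick accumulates an angle from the rotation speed and clockwise flag, then RotateActorAroundPoint places the hammer at that angle and radius around the target's current location.
; It moves only while the target is valid, without sweeping.
; Sphere overlaps apply fixed damage to any actor other than player 0's pawn.
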(event `self.ReceiveBeginPlay`
  ;[1 1 1] 위치
  (set `self.ActorPosition` (`self.K2_GetActorLocation`)))

(event `self.ReceiveTick`
  (params (DeltaSeconds :type "Float (single-precision)"))
  ;[1 1 1] 내 주위 멤돌아
  (set `self.ActerRotation` (+ (`self.ActerRotation`) (* (* DeltaSeconds (`self.RotationSpeed`)) (`KismetMathLibrary.SelectFloat` 1.0 -1.0 (`self.Clockwise`)))))
  (`self.RotateActorAroundPoint` self (`self.TargetActor`) (`self.ActorPosition`) (`self.Radius`) (`self.StartingAngle`) (`self.ActerRotation`)))

(event `self.Sphere.OnComponentBeginOverlap`
  (params (OverlappedComponent :type "PrimitiveComponent Object Reference") (OtherActor :type "Actor Object Reference") (OtherComp :type "PrimitiveComponent Object Reference") (OtherBodyIndex :type Integer) (bFromSweep :type Boolean) (SweepResult :type "HitResult Structure (by ref)"))
  ;[1 1 1] 데미지
  (if (not (== OtherActor (`GameplayStatics.GetPlayerPawn` 0)))
    (`GameplayStatics.ApplyDamage` OtherActor 50.0)))

(fn `RotateActorAroundPoint`
  (params (ActorToRotate :type "Actor Object Reference") (TargetActor :type "Actor Object Reference") (TargetLocation :type "Vector Structure") (Radius :type "Float (double-precision)") (Angle :type "Float (double-precision)") (RotationRate :type "Float (double-precision)"))
  (returns (NewParam :type "Vector Structure"))
  (locals (LActorToRotate :type "Actor Object Reference") (LTargetActor :type "Actor Object Reference") (LLocation :type "Vector Structure") (LoRadius :type "Float (double-precision)") (LAngle :type "Float (double-precision)") (LRate :type "Float (double-precision)"))
  (set `local.LActorToRotate` ActorToRotate)
  (set `local.LTargetActor` TargetActor)
  (set `local.LLocation` TargetLocation)
  (set `local.LoRadius` Radius)
  (set `local.LAngle` Angle)
  (set `local.LRate` RotationRate)
  (`/Engine/EditorBlueprintResources/StandardMacros.IsValid` (`local.LTargetActor`)
    (:`Is Valid`
      (set `local.LLocation` (`self.K2_GetActorLocation` (`local.LTargetActor`)))
      (`self.K2_SetActorLocation` (`local.LActorToRotate`) (+ (`local.LLocation`) (`KismetMathLibrary.RotateAngleAxis` (`KismetMathLibrary.MakeVector` (`local.LoRadius`)) (+ (`local.LRate`) (`local.LAngle`)) (0.0 0.0 1.0))) false false)
      (return (`local.LLocation`)))))

(fn `UserConstructionScript`)