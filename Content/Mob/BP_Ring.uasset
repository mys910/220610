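; BP_Ring is a mob-side actor that homes in on player 0's pawn and destroys itself after a short lifetime.
; BeginPlay caches the pawn, snaps to face it and starts a timer that calls RingClear to destroy the ring.
; Each Tick blends rotation toward the target and moves forward by a fixed, frame-rate-dependent step without sweeping.
; The graphs contain no hit or damage logic.
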(event `self.ReceiveBeginPlay`
  (set `self.TargetActor` (`GameplayStatics.GetPlayerPawn` 0))
  (`self.K2_SetActorRotation` (`KismetMathLibrary.FindLookAtRotation` (`self.K2_GetActorLocation`) (`self.K2_GetActorLocation` (`self.TargetActor`))))
  (`KismetSystemLibrary.K2_SetTimer` null "RingClear" 5.0))

(event `self.ReceiveTick`
  (params (DeltaSeconds :type "Float (single-precision)"))
  (bind _targetactor (`self.TargetActor`))
  (`/Engine/EditorBlueprintResources/StandardMacros.IsValid` _targetactor
    (:`Is Valid`
      (`self.K2_SetActorRotation` (`KismetMathLibrary.RLerp` (`self.K2_GetActorRotation`) (`KismetMathLibrary.FindLookAtRotation` (`self.K2_GetActorLocation`) (`self.K2_GetActorLocation` _targetactor)) 0.1 true))
      (`self.K2_AddActorWorldOffset` (* (`self.GetActorForwardVector`) 50.0)))))

(fn `RingClear`
  (`self.K2_DestroyActor`))

(fn `UserConstructionScript`)