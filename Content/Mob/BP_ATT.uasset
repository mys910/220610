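; BP_ATT is a short-lived attack actor that moves through the level and damages actors it overlaps, except the player pawn.
; On BeginPlay it rotates to face the player and starts a brief timer that calls AttClear to destroy it.
; Each Tick it moves at a fixed per-frame step along its up vector, not its forward vector, without sweeping.
; Box overlaps apply fixed damage without destroying the actor.
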(event `self.ReceiveBeginPlay`
  (bind _returnvalue (`GameplayStatics.GetPlayerPawn` 0))
  ;[1 1 1] 액터 생성
  (set `self.TargetActor` _returnvalue)
  (`self.K2_SetActorRotation` (`KismetMathLibrary.FindLookAtRotation` (`self.K2_GetActorLocation`) (`self.K2_GetActorLocation` _returnvalue)))
  (`KismetSystemLibrary.K2_SetTimer` null "AttClear" 0.2))

(event `self.ReceiveTick`
  (params (DeltaSeconds :type "Float (single-precision)"))
  ;[1 1 1] 액터 발사
  (`/Engine/EditorBlueprintResources/StandardMacros.IsValid` (`self.TargetActor`)
    (:`Is Valid`
      (`self.K2_SetActorRotation` (`self.K2_GetActorRotation`))
      (`self.K2_AddActorWorldOffset` (* (`self.GetActorUpVector`) 20.0)))))

(event `self.Box.OnComponentBeginOverlap`
  (params (OverlappedComponent :type "PrimitiveComponent Object Reference") (OtherActor :type "Actor Object Reference") (OtherComp :type "PrimitiveComponent Object Reference") (OtherBodyIndex :type Integer) (bFromSweep :type Boolean) (SweepResult :type "HitResult Structure (by ref)"))
  ;[1 1 1] ATT 데미지
  (if (not (== OtherActor (`GameplayStatics.GetPlayerPawn` 0)))
    (`GameplayStatics.ApplyDamage` OtherActor 20.0)))

(fn `AttClear`
  (`self.K2_DestroyActor`))

(fn `UserConstructionScript`)