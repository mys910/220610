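; BP_MobLevel1 is an enemy mob that chases the player pawn and drops a BP_Potion when killed.
; Each Tick it slowly lerps its rotation toward the player and moves forward by an unswept, frame-rate-dependent offset.
; AnyDamage lowers HP and updates the Widget_HP bar, with death handled only while that widget is valid.
; Box overlaps and mesh hits apply fixed damage to any other actor involved.
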(event `self.ReceiveBeginPlay`
  ;[1 1 1] 액터생성
  (set `self.TargetActor` (`GameplayStatics.GetPlayerPawn` 0))
  (`self.K2_SetActorRotation` (`KismetMathLibrary.FindLookAtRotation` (`self.K2_GetActorLocation`) (`self.K2_GetActorLocation` (`self.TargetActor`))))
  ;[1 1 1] 몹 HP 스폰
  (bind _aswidget_hp (cast `/Game/UI/Widget_HP` (`WidgetComponent.GetUserWidgetObject` (`self.HP_Bar`))))
  (bind _output_get (set `self.HP_Bar_UI` _aswidget_hp))
  (set `/Game/UI/Widget_HP.EnergyPercent` (/ (`self.HP`) (`self.MAX_HP`)) _output_get))

(event `self.ReceiveTick`
  (params (DeltaSeconds :type "Float (single-precision)"))
  (bind _targetactor (`self.TargetActor`))
  ;[1 1 1] 액터 따라오기
  (`/Engine/EditorBlueprintResources/StandardMacros.IsValid` _targetactor
    (:`Is Valid`
      (`self.K2_SetActorRotation` (`KismetMathLibrary.RLerp` (`self.K2_GetActorRotation`) (`KismetMathLibrary.FindLookAtRotation` (`self.K2_GetActorLocation`) (`self.K2_GetActorLocation` _targetactor)) 0.01 true))
      (`self.K2_AddActorWorldOffset` (* (`self.GetActorForwardVector`) 1.0)))))

(event `self.ReceiveAnyDamage`
  (params (Damage :type "Float (single-precision)") (DamageType :type "DamageType Object Reference") (InstigatedBy :type "Controller Object Reference") (DamageCauser :type "Actor Object Reference"))
  (bind _hp_bar_ui (`self.HP_Bar_UI`))
  ;[1 1 1] 몹 데미지 받기
  (set `self.HP` (- (`self.HP`) Damage))
  (`/Engine/EditorBlueprintResources/StandardMacros.IsValid` _hp_bar_ui
    (:`Is Valid`
      (set `/Game/UI/Widget_HP.EnergyPercent` (/ (`self.HP`) (`self.MAX_HP`)) _hp_bar_ui)
      (if (<= (`self.HP`) 0.0)
        ;[1 1 1] 아이템 드랍
        (`|SpawnActorFromClass` "/Game/Mob/BP_Potion.BP_Potion_C" (`SceneComponent.K2_GetComponentToWorld` (`self.Mesh`)) "Undefined" "OverrideRootScale" null null)
        (`self.K2_DestroyActor`)))))

(event `self.Box.OnComponentBeginOverlap`
  (params (OverlappedComponent :type "PrimitiveComponent Object Reference") (OtherActor :type "Actor Object Reference") (OtherComp :type "PrimitiveComponent Object Reference") (OtherBodyIndex :type Integer) (bFromSweep :type Boolean) (SweepResult :type "HitResult Structure (by ref)"))
  ;[1 1 1] 몹 데미지
  (`GameplayStatics.ApplyDamage` OtherActor 10.0))

(event `self.Mesh.OnComponentHit`
  (params (HitComponent :type "PrimitiveComponent Object Reference") (OtherActor :type "Actor Object Reference") (OtherComp :type "PrimitiveComponent Object Reference") (NormalImpulse :type "Vector Structure") (Hit :type "HitResult Structure (by ref)"))
  ;[1 1 1] 몹 데미지
  (`GameplayStatics.ApplyDamage` OtherActor 10.0))

(fn `UserConstructionScript`)